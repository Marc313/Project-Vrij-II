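; BP_Projectile is an enemy-fired projectile that damages the player character, or enemies once reflected.
; Tick moves it along its direction without sweep, turns its sprite toward the camera and destroys it when its lifetime expires.
; Reflect stops the lifetime countdown and boosts speed, which then keeps growing while steering blends from away from the reflect point toward the owner enemy by relative distances.
; Sphere overlap applies the hit and destroys it.
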(event OnComponentBeginOverlap(Sphere)
  (params (OverlappedComponent :type Primitive%20Component%20Object%20Reference) (OtherActor :type Actor%20Object%20Reference) (OtherComp :type Primitive%20Component%20Object%20Reference) (OtherBodyIndex :type Integer) (bFromSweep :type Boolean) (SweepResult :type Hit%20Result%20Structure%20%28by%20ref%29))
  (if (Variables|Default|GetisReflected)
    (bind _asbp_enemy_base (Utilities|Casting|CastToBP_EnemyBase OtherActor))
    (Default|OnHit _asbp_enemy_base (* (Variables|Default|GetReflectionDamageMultiplier) (Variables|Default|GetProjectileDamage)))
    (Actor|DestroyActor)
    (else
      (bind _asbp_combat_character (Utilities|Casting|CastToBP_Combat_Character OtherActor))
      (Default|OnHit _asbp_combat_character (Variables|Default|GetProjectileDamage))
      (Actor|DestroyActor))))

(event EventBeginPlay
  (Variables|Default|SetCurrentLifetime (Variables|Default|GetMaxLifetime)))

(event EventTick
  (params (DeltaSeconds :type Float%20%28single-precision%29))
  (Utilities|FlowControl|Sequence
    (:then_0
      (if (Variables|Default|GetisReflected)
        (CallFunction|CalculateDirectiontoTarget (Variables|Default|GetOwnerEnemy))
        (Variables|Default|SetMoveSpeed (* (+ 1.0 (* (Variables|Default|GetReflectionLifeTimeSpeedMultiplier) DeltaSeconds)) (Variables|Default|GetMoveSpeed)))))
    (:then_1
      (CallFunction|MovetoDirection DeltaSeconds)
      (CallFunction|SetWidgetRotation)
      (if (not (Variables|Default|GetisReflected))
        (bind _output_get (Variables|Default|SetCurrentLifetime (- (Variables|Default|GetCurrentLifetime) DeltaSeconds)))
        (if (<= _output_get 0.0)
          (Actor|DestroyActor))))))

(fn ConstructionScript)

(fn SetDirection
  (params (Direction :type Vector))
  (Variables|Default|SetDirection Direction))

(fn MovetoDirection
  (params (Delta%20Seconds :type Float%20%28double-precision%29))
  (Transformation|SetWorldLocation (Variables|Default|GetDefaultSceneRoot) (+ (Transformation|GetWorldLocation (Variables|Default|GetDefaultSceneRoot)) (* (Variables|Default|GetDirection) (Variables|Default|GetMoveSpeed) Delta%20Seconds)) false false))

(fn SetWidgetRotation
  (bind _sprite (Variables|Default|GetSprite))
  (Utilities|IsValid _sprite
    (:Is%20Valid
      (Transformation|SetWorldRotation _sprite (Math|Rotator|FindLookatRotation (Transformation|GetWorldLocation _sprite) (Transformation|GetWorldLocation (Variables|/Script/Engine.PlayerCameraManager|GetTransformComponent (Game|GetPlayerCameraManager 0)))) false false))))

(fn Reflect
  (params (PlayerPos :type Vector))
  (Variables|Default|SetReflectPos PlayerPos)
  (Variables|Default|SetisReflected true)
  (Variables|Default|SetMoveSpeed (* (Variables|Default|GetMoveSpeed) (Variables|Default|GetReflectionSpeedMultiplier))))

(fn CalculateDirectiontoTarget
  (params (Target :type Actor%20Object%20Reference))
  (bind _returnvalue (Transformation|GetActorLocation Target))
  (bind _returnvalue_2 (Transformation|GetActorLocation))
  (bind _returnvalue_3 (Transformation|GetActorLocation))
  (bind _reflectpos (Variables|Default|GetReflectPos))
  (bind _returnvalue_4 (Math|Vector|MakeVector (.x _reflectpos) (.y _reflectpos) (.z _returnvalue_2)))
  (bind _returnvalue_5 (Math|Vector|MakeVector (.x _returnvalue_2) (.y _returnvalue_2) (.z _returnvalue_2)))
  (bind _returnvalue_6 (Math|Vector|Distance(Vector) _returnvalue_5 _returnvalue_4))
  (Variables|Default|SetDirection (Math|Vector|Lerp(Vector) (Math|Vector|Normalize (- _returnvalue_5 _returnvalue_4)) (Math|Vector|Normalize (- _returnvalue _returnvalue_3)) (/ _returnvalue_6 (+ (* (Math|Vector|Distance(Vector) _returnvalue _returnvalue_3) 1.5) _returnvalue_6)))))

(fn SetOwnerEnemy
  (params (Owner :type Actor%20Object%20Reference))
  (Variables|Default|SetOwnerEnemy Owner))