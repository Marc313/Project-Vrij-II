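; Player character for the room that creates the HUD canvas, toggles its interact text, and can hand control to the combat character for the arena.
; BeginPlay caches the combat character, and the 0 key triggers SwitchToArena, which removes input mapping, possesses that character and hides the prompt.
; OnPossess restores input mapping and shows the win widget if exactly one Afvalhoop_Base actor exists, otherwise printing a debug message.
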(event EventBeginPlay
  (|CallParentFunction)
  (Utilities|FlowControl|Sequence
    (:then_0
      ;[1 1 1] Create Canvas Widget
      (bind _returnvalue (UserInterface|CreateWidget "/Game/_04_UI/HUD_Canvas.HUD_Canvas_C" (Game|GetPlayerController 0)))
      (bind _output_get (Variables|Default|SetHUD_Canvas _returnvalue))
      (UserInterface|Viewport|AddtoViewport _output_get 0))
    (:then_1
      (bind _returnvalue_2 (Actor|GetActorOfClass "/Game/_01_Dev/BP_Combat_Character.BP_Combat_Character_C"))
      (Variables|Default|SetCombat_Character _returnvalue_2))))

(event Input|KeyboardEvents|0
  (params (Key :type Key%20Structure :default "None"))
  (:Pressed
    (CallFunction|SwitchtoArena)))

(fn ConstructionScript
  (|CallParentFunction))

(fn SwitchtoArena
  (bind _combat_character (Variables|Default|GetCombat_Character))
  (CallFunction|RemoveInputMapping)
  (Pawn|Possess (Game|GetPlayerController 0) _combat_character)
  (Default|OnPossess _combat_character)
  (CallFunction|ShowInteractText false))

(fn ShowInteractText
  (params (Show :type Boolean))
  (Default|ShowInteractText (Variables|Default|GetHUD_Canvas) Show))

(fn OnPossess
  (CallFunction|AddInputMapping)
  (bind _outactors (Actor|GetAllActorsOfClass "/Game/_01_Dev/Interactable/Afvalhoop_Base.Afvalhoop_Base_C"))
  (if (== (Utilities|Array|Length _outactors) 1)
    (bind _returnvalue (UserInterface|CreateWidget "/Game/_04_UI/Win_Box.Win_Box_C" (Game|GetPlayerController 0)))
    (UserInterface|Viewport|AddtoViewport _returnvalue 0)
    (else
      (Development|PrintString "Not yet"))))