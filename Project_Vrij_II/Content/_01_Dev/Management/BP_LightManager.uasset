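; Level light manager that changes the directional light's rotation as the player completes levels.
; On BeginPlay it applies a default rotation and binds to the completion events of Level1 and Level2.
; Each completion snaps the light to that level's preset rotation through SetLightRotation.
; An additive rotation variant, SetLightRotationWithValue, remains in the graph, but its event bindings never run.
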(event Custom|OnLevelCompleted_Event
  (CallFunction|SetLightRotationwithValue))

(event Custom|SetLight1
  (CallFunction|SetLightRotation (Variables|Default|GetAfter1Rotation)))

(event Custom|SetLight2
  (CallFunction|SetLightRotation (Variables|Default|GetAfter2Rotation)))

(event EventBeginPlay
  (CallFunction|SetLightRotation (Variables|Default|GetDefaultRotation))
  (EventDispatchers|AssignOnLevelCompleted (Variables|Default|GetLevel1) (delegate Custom|SetLight1))
  (EventDispatchers|BindEventtoOnLevelCompleted (Variables|Default|GetLevel2) (delegate Custom|SetLight2)))

(fn ConstructionScript)

(fn SetLightRotationwithValue
  (bind _afterlevel1rot (Variables|Default|GetAfterLevel1Rot))
  (bind _directionallight (Variables|Default|GetDirectionalLight))
  (bind _returnvalue (Transformation|GetActorRotation _directionallight))
  (Transformation|SetActorRotation _directionallight (Math|Rotator|MakeRotator (+ _afterlevel1rot (.roll _returnvalue)) (+ (.pitch _returnvalue) _afterlevel1rot) (+ (.yaw _returnvalue) _afterlevel1rot))))

(fn SetLightRotation
  (params (Rotation :type Rotator))
  (Transformation|SetActorRotation (Variables|Default|GetDirectionalLight) Rotation))