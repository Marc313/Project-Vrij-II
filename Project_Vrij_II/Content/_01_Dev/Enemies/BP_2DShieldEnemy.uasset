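; BP_2DShieldEnemy is a 2D sprite enemy whose shield absorbs hits before its health takes damage.
; OnHit drains the shield while blocking, updates its healthbar widget and plays a sound whose pitch parameter rises as the shield weakens.
; Breaking the shield hides the bar and passes hits to the parent, until enough further health loss restores it fully.
; Blackboard flags report shield hits and breaks to the AI.
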(event EventBeginPlay
  (|CallParentFunction)
  (Utilities|FlowControl|Sequence
    (:then_0
      (Variables|Blocking|SetShieldHealth (Variables|Blocking|GetMaxShieldHealth)))
    (:then_1
      (bind _asmisc_healthbar (Utilities|Casting|CastToMisc_Healthbar (UserInterface|GetWidget (Variables|Default|GetShield_Healthbar))))
      (Variables|Default|SetShieldBarUI (Variables|/Game/_04_UI/Misc_Healthbar.Misc_Healthbar_C|GetHealthbar _asmisc_healthbar)))))

(event EventTick
  (params (DeltaSeconds :type Float%20%28single-precision%29))
  (|CallParentFunction DeltaSeconds)
  (CallFunction|SetWidgetRotation (Variables|Default|GetWidget))
  (CallFunction|SetWidgetRotation (Variables|Default|GetEnemy_Sprite))
  (CallFunction|SetWidgetRotation (Variables|Default|GetShield_Healthbar)))

(fn ConstructionScript
  (|CallParentFunction))

(fn OnHit
  (params (Damage :type Float%20%28double-precision%29))
  (if (Variables|Blocking|GetIsBlocking)
    (CallFunction|OnShieldHit Damage)
    (else
      (|CallParentFunction Damage)
      (if (>= (- (Variables|Default|GetHealthOnShieldBreak) (Variables|Default|GetHealth)) 1e+02)
        (CallFunction|RegainShield)))))

(fn OnShieldHit
  (params (Damage :type Float%20%28double-precision%29))
  (Utilities|FlowControl|Sequence
    (:then_0
      (if (<= (- (Variables|Blocking|GetShieldHealth) Damage) 0.0)
        (CallFunction|OnShieldBreak)
        (else
          (bind _output_get (Variables|Blocking|SetShieldHealth (- (Variables|Blocking|GetShieldHealth) Damage)))
          (Development|PrintString (Utilities|String|Append (Utilities|String|MakeLiteralString "Health: ") (Utilities|String|ToString(Float) _output_get)))
          (CallFunction|UpdateShieldbar))))
    (:then_1
      (bind _output_get_2 (Variables|Default|SetPitchInput (- 1.0 (/ (Variables|Blocking|GetShieldHealth) (Variables|Blocking|GetMaxShieldHealth)))))
      (bind _returnvalue (Audio|CreateSound2D "/Game/_07_Audio/SFX/_Shield_Cue._Shield_Cue" 1.0 1.0 0.0 0))
      (Audio|Parameter|SetFloatParameter _returnvalue "Pitch" _output_get_2 :!class /Script/AudioExtensions.AudioParameterControllerInterface)
      (Audio|Components|Audio|Play _returnvalue 0.0))
    (:then_2
      (AI|Components|Blackboard|SetValueasBool (AI|GetBlackboard (AI|GetAIController self)) (Utilities|Name|MakeLiteralName "IsHit") true))))

(fn OnShieldBreak
  (Rendering|SetVisibility (Variables|Default|GetShield_Healthbar) false true)
  (Variables|Blocking|SetIsBlocking false)
  (AI|Components|Blackboard|SetValueasBool (AI|GetBlackboard (AI|GetAIController self)) (Utilities|Name|MakeLiteralName "IsShieldBroken") true)
  (Variables|Default|SetHealthOnShieldBreak (Variables|Default|GetHealth))
  (Audio|PlaySound2D "/Game/_07_Audio/SFX/_ShieldBreak_Cue._ShieldBreak_Cue" 1.0 1.0 0.0 0 0))

(fn UpdateShieldbar
  (Progress|SetPercent (Variables|Default|GetShieldBarUI) (/ (Variables|Blocking|GetShieldHealth) (Variables|Blocking|GetMaxShieldHealth))))

(fn RegainShield
  (Rendering|SetVisibility (Variables|Default|GetShield_Healthbar) true true)
  (Variables|Blocking|SetIsBlocking true)
  (AI|Components|Blackboard|SetValueasBool (AI|GetBlackboard (AI|GetAIController self)) (Utilities|Name|MakeLiteralName "IsShieldBroken") false)
  (Variables|Blocking|SetShieldHealth (Variables|Blocking|GetMaxShieldHealth))
  (CallFunction|UpdateShieldbar))