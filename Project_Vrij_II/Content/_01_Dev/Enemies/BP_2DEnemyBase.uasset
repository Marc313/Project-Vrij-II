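; Base Blueprint for a 2D enemy whose sprite is displayed through a widget component.
; Sprites are swapped on the widget's image by list index or direct reference; direct requests during a timed lock are remembered, with the latest applied when it expires.
; On hit, a timeline flashes the widget red and restores its original color, while the AI controller's blackboard IsHit flag is set.
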(event Custom|HitImpactEvent
  (bind _enemy_sprite (Variables|Default|GetEnemy_Sprite))
  (bind _returnvalue (UserInterface|GetWidget _enemy_sprite))
  (bind _color (Timeline|Timeline PlayFromStart)
    (:Update
      (Appearance|SetColorandOpacity _returnvalue (Math|Color|Lerp(LinearColor) (Variables|Default|GetOriginalColor) "(R=1.000000,G=0.041156,B=0.071003,A=1.000000)" _color) :!class /Script/UMG.UserWidget))
    (:Finished
      (Appearance|SetColorandOpacity _returnvalue (Variables|Default|GetOriginalColor) :!class /Script/UMG.UserWidget))))

(event EventBeginPlay
  (|CallParentFunction)
  (Variables|Default|SetOriginalColor (Variables|/Script/UMG.UserWidget|GetColorAndOpacity (UserInterface|GetWidget (Variables|Default|GetEnemy_Sprite)))))

(event EventTick
  (params (DeltaSeconds :type Float%20%28single-precision%29))
  (|CallParentFunction DeltaSeconds))

(fn ConstructionScript
  (|CallParentFunction))

(fn SetEnemySpritewithIndex
  (params (Index :type Integer))
  (bind _enemyspritelist (Variables|Default|GetEnemySpriteList))
  (if (Utilities|Array|IsValidIndex _enemyspritelist Index)
    (bind _astest_enemy (Utilities|Casting|CastToTestEnemy (UserInterface|GetWidget (Variables|Default|GetEnemy_Sprite))))
    (bind _newparam (Default|GetImage _astest_enemy))
    (Class|Image|SetBrush _newparam (Class|PaperSpriteBlueprintLibrary|MakeBrushfromSprite (Utilities|Array|Get(acopy) _enemyspritelist Index)))))

(fn OnHit
  (params (Damage :type Float%20%28double-precision%29))
  (|CallParentFunction Damage)
  (CallFunction|HitImpactEvent)
  (AI|Components|Blackboard|SetValueasBool (AI|GetBlackboard (AI|GetAIController self)) (Utilities|Name|MakeLiteralName "IsHit") true))

(fn SetEnemySprite
  (params (Sprite :type Paper%20Sprite%20Object%20Reference))
  (Variables|Default|SetRecentSpriteRequest Sprite)
  (if (Variables|Default|GetSpriteSwitchAvailable)
    (bind _astest_enemy (Utilities|Casting|CastToTestEnemy (UserInterface|GetWidget (Variables|Default|GetEnemy_Sprite))))
    (bind _newparam (Default|GetImage _astest_enemy))
    (Class|Image|SetBrush _newparam (Class|PaperSpriteBlueprintLibrary|MakeBrushfromSprite Sprite))))

(fn DisableSpriteSwitch
  (params (Duration :type Float%20%28double-precision%29))
  (Variables|Default|SetSpriteSwitchAvailable false)
  (Utilities|Time|SetTimerbyFunctionName 0 "EnableSpriteSwitch" Duration))

(fn EnableSpriteSwitch
  (Variables|Default|SetSpriteSwitchAvailable true)
  (Utilities|IsValid (Variables|Default|GetRecentSpriteRequest)
    (:Is%20Valid
      (CallFunction|SetEnemySprite (Variables|Default|GetRecentSpriteRequest))
      (Variables|Default|SetRecentSpriteRequest 0))))