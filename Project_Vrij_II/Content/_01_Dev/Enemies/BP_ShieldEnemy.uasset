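; BP_ShieldEnemy is an enemy whose shield absorbs hits while it is blocking.
; OnHit sends damage to a separate shield health pool when IsBlocking, otherwise to the parent's OnHit.
; Surviving shield hits update a widget health bar and print the remaining value.
; A breaking hit hides the shield, clears blocking and sets the AI blackboard's IsShieldBroken key, without passing on excess damage.
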(event EventBeginPlay
  (|CallParentFunction)
  (Utilities|FlowControl|Sequence
    (:then_0
      (Variables|Blocking|SetShieldHealth (Variables|Blocking|GetMaxShieldHealth)))
    (:then_1
      (bind _asmisc_healthbar (Utilities|Casting|CastToMisc_Healthbar (UserInterface|GetWidget (Variables|Default|GetShield_Healthbar))))
      (Variables|Default|SetShieldBarUI (Variables|/Game/_04_UI/Misc_Healthbar.Misc_Healthbar_C|GetHealthbar _asmisc_healthbar)))))

(event EventTick
  (params (DeltaSeconds :type Float%20%28single-precision%29))
  (|CallParentFunction DeltaSeconds) ; This node is disabled and will not be called.\nDrag off pins to build functionality.
)

(fn ConstructionScript
  (|CallParentFunction))

(fn OnHit
  (params (Damage :type Float%20%28double-precision%29))
  (if (Variables|Blocking|GetIsBlocking)
    (CallFunction|OnShieldHit Damage)
    (else
      (|CallParentFunction Damage))))

(fn OnShieldHit
  (params (Damage :type Float%20%28double-precision%29))
  (if (<= (- (Variables|Blocking|GetShieldHealth) Damage) 0.0)
    (CallFunction|OnShieldBreak)
    (else
      (bind _output_get (Variables|Blocking|SetShieldHealth (- (Variables|Blocking|GetShieldHealth) Damage)))
      (Development|PrintString (Utilities|String|Append (Utilities|String|MakeLiteralString "Health: ") (Utilities|String|ToString(Float) _output_get)))
      (CallFunction|UpdateShieldbar))))

(fn OnShieldBreak
  (Rendering|SetVisibility (Variables|Default|GetShield) false true)
  (Variables|Blocking|SetIsBlocking false)
  (AI|Components|Blackboard|SetValueasBool (AI|GetBlackboard (AI|GetAIController self)) (Utilities|Name|MakeLiteralName "IsShieldBroken") true))

(fn UpdateShieldbar
  (Progress|SetPercent (Variables|Default|GetShieldBarUI) (/ (Variables|Blocking|GetShieldHealth) (Variables|Blocking|GetMaxShieldHealth))))