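; BP_EnemyBase is an enemy base Blueprint that tracks health and dies when it runs out.
; BeginPlay sets Health to MaxHealth, and OnHit subtracts damage, printing the remaining health or printing a death message and destroying the actor once it would reach zero or below.
; A P key binding applies a fixed hit through OnHit, apparently as a debug trigger.
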(event EventBeginPlay
  (Variables|Default|SetHealth (Variables|Default|GetMaxHealth)))

(event Collision|EventActorBeginOverlap
  (params (OtherActor :type Actor%20Object%20Reference)))

(event EventTick
  (params (DeltaSeconds :type Float%20%28single-precision%29)))

(event Input|KeyboardEvents|P
  (params (Key :type Key%20Structure :default "None"))
  (:Pressed
    (CallFunction|OnHit 3e+01)
    (Development|PrintString "P")))

(fn ConstructionScript)

(fn OnHit
  (params (Damage :type Float%20%28double-precision%29))
  (if (<= (- (Variables|Default|GetHealth) Damage) 0.0)
    (Development|PrintString "The enemy died" (<= (- (Variables|Default|GetHealth) Damage) 0.0))
    (Actor|DestroyActor)
    (else
      (bind _output_get (Variables|Default|SetHealth (- (Variables|Default|GetHealth) Damage)))
      (Development|PrintString (Utilities|String|Append (Utilities|String|MakeLiteralString "Health: ") (Utilities|String|ToString(Float) _output_get))))))